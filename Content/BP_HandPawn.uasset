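; VR player pawn that sets a floor-level tracking origin and provides the player's left and right hands.
; On BeginPlay it spawns BP_Hand for the left and BP_RightHand, with its Hand set to Right, for the right, owning and storing both.
; Each hand actor is attached to the pawn, snapping location and rotation while keeping world scale.
; The pawn has no tick or overlap logic.
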(event EventBeginPlay
  (bind _returnvalue (Math|Transform|MakeTransform "0, 0, 0"))
  (bind _self self)
  (bind _self_2 self)
  (Utilities|FlowControl|Sequence
    (:then_0
      (Class|HeadMountedDisplayFunctionLibrary|SetTrackingOrigin "Floor"))
    (:then_1
      (Utilities|FlowControl|Sequence
        (:then_0
          (bind _returnvalue_2 (Game|SpawnActorfromClass "/Game/BP_Hand.BP_Hand_C" _returnvalue "Undefined" _self "Left" 0))
          (bind _output_get (Variables|Default|SetLeftHand _returnvalue_2))
          (Transformation|AttachActorToActor _output_get _self_2 "None" "SnapToTarget" "SnapToTarget" "KeepWorld" false))
        (:then_1
          (bind _returnvalue_3 (Game|SpawnActorfromClass "/Game/BP_RightHand.BP_RightHand_C" _returnvalue "Undefined" _self "Right" 0))
          (bind _output_get_2 (Variables|Default|SetRightHand _returnvalue_3))
          (Transformation|AttachActorToActor _output_get_2 _self_2 "None" "SnapToTarget" "SnapToTarget" "KeepWorld" false))))))

(event Collision|EventActorBeginOverlap
  (params (OtherActor :type Actor%20Object%20Reference)))

(event EventTick
  (params (DeltaSeconds :type Float%20%28single-precision%29)))

(fn ConstructionScript)